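; Player character Blueprint that handles dashing, pausing, HUD creation and death reporting.
; Dash launches a moving character along its horizontal velocity scaled up, then clears CanDash to prevent chaining; this file never resets the flag.
; BeginPlay adds the HUD, while Pause lazily creates and reuses a menu widget, switches to UI-only input and pauses the game.
; PlayerDied forwards to the GameInstance's death handler.
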(event EventBeginPlay
  (CallFunction|SetupHUD))

(event EventPlayerDied
  (CallFunction|HandlePlayerDeath))

(event Input|ActionEvents|InputActionDash
  (params (Key :type Key%20Structure :default "AnyKey"))
  (:Pressed
    (CallFunction|HandleDash)))

(event Input|ActionEvents|InputActionPause
  (params (Key :type Key%20Structure :default "AnyKey"))
  (:Pressed
    (CallFunction|HandlePause)))

(fn ConstructionScript
  (|CallParentFunction))

(fn HandleDash
  (bind _returnvalue (Transformation|GetVelocity))
  (if (Variables|Default|GetbCanDash)
    (if (Math|Vector|NotEqual(Vector) _returnvalue "0, 0,0.000000" 0.0001)
      (Character|LaunchCharacter (* (+ _returnvalue "0, 0, 0") "2.500000,2.500000, 0") false false)
      (Variables|Default|SetbCanDash false) ; Prevent Chain Dashing
    )))

(fn HandlePlayerDeath
  (bind _asbp_game_instance (Utilities|Casting|CastToBP_GameInstance (Game|GetGameInstance)))
  (Default|PlayerDiedEventHandler _asbp_game_instance))

(fn SetupHUD
  (bind _returnvalue (UserInterface|CreateWidget "/Game/UI/Blueprints/BP_HUD.BP_HUD_C"))
  (bind _output_get (Variables|Default|SetHUDReference _returnvalue))
  (UserInterface|Viewport|AddtoViewport _output_get 0))

(fn HandlePause
  (bind _returnvalue (Game|GetPlayerController 0))
  (Utilities|IsValid (Variables|Default|GetPauseMenuReference)
    (:Is%20Valid
      _)
    (:Is%20Not%20Valid
      (bind _returnvalue_2 (UserInterface|CreateWidget "/Game/UI/Blueprints/BP_PauseMenu.BP_PauseMenu_C" _returnvalue))
      (bind _output_get (Variables|Default|SetPauseMenuReference _returnvalue_2))))
  (Input|SetInputModeUIOnly _returnvalue _output_get "DoNotLock")
  (UserInterface|Viewport|AddtoViewport _output_get 0)
  (Game|SetGamePaused true))